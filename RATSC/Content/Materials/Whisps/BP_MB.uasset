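; BP_MB is a Blueprint meant to shuttle its Cube component back and forth between its starting relative location and EndLocationHorizontal.
; BeginPlay stores the start location, then chains two MoveComponentTo calls in an endless loop, each leg timed by Speed.
; The loop is gated by a cast of Cube to AnimNotifyState_Trail, which a scene component cannot satisfy, so the movement never starts as written.
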(event `self.ReceiveBeginPlay`
  (bind _speed (`self.Speed`))
  (bind _cube (`self.Cube`))
  (cast `AnimNotifyState_Trail` (`self.Cube`))
  (set `self.EndLocationHorizontal` (+ (`self.EndLocationHorizontal`) (0.0 0.0 0.0)))
  (set `self.StartLocation` (`SceneComponent.RelativeLocation` _cube))
  (`KismetSystemLibrary.MoveComponentTo` _cube (`self.EndLocationHorizontal`) (struct) false false _speed :!label _label)
  (`KismetSystemLibrary.MoveComponentTo` _cube (`self.StartLocation`) (struct) false false _speed)
  (goto _label))

(fn `UserConstructionScript`)