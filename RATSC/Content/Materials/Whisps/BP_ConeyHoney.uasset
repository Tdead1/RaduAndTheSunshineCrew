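; BP_ConeyHoney is an actor with a Cylinder component that marks the tree closest to the player's camera, likely as a wisp-style visual.
; Every tick it finds the BP_CameraController and moves itself to the location of the ClosestTree reported by its ACTreeDetection component, without a validity check.
; It also hides or shows the cylinder each tick, hiding it while BP_PlayerController is in one specific CurrentState.
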(event `self.ReceiveTick`
  (params (DeltaSeconds :type "Float (single-precision)"))
  (bind _outactors (`GameplayStatics.GetAllActorsOfClass` "/Game/Player/BP_CameraController.BP_CameraController_C"))
  (`SceneComponent.SetHiddenInGame` (`self.Cylinder`) (`|EnumEquality` (`/Game/Player/BP_PlayerController.CurrentState` (cast `/Game/Player/BP_PlayerController` (`GameplayStatics.GetPlayerController` 0) :!pure true)) "NewEnumerator2") false)
  (`self.K2_SetActorLocation` (`self.K2_GetActorLocation` (`/Game/Player/AC_TreeDetection.ClosestTree` (`/Game/Player/BP_CameraController.AC_TreeDetection` (`|GetArrayItem` _outactors))))))

(fn `UserConstructionScript`)