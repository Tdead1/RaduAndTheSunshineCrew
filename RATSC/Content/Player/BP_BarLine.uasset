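; BP_BarLine is a player-related effect that shows beam particle lines reaching to the character, scaled by a takeover counter.
; Every Tick it re-aims nine beam emitters at the character's location and pins most of their sources to the zero vector.
; Counter thresholds then toggle visibility between all lines and the first four.
; The single-line tier repeats the middle threshold, so it never runs, and low counts leave visibility unchanged.
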(event `self.ReceiveTick`
  (params (DeltaSeconds :type "Float (single-precision)"))
  (bind _p_barline (`self.P_BarLine`))
  (`ParticleSystemComponent.SetBeamTargetPoint` _p_barline 0 (`self.K2_GetActorLocation` (`self.Character`)) 0)
  (`ParticleSystemComponent.SetBeamTargetPoint` (`self.P_BarLine2`) 0 (`self.K2_GetActorLocation` (`self.Character`)) 0)
  (`ParticleSystemComponent.SetBeamTargetPoint` (`self.P_BarLine3`) 0 (`self.K2_GetActorLocation` (`self.Character`)) 0)
  (`ParticleSystemComponent.SetBeamTargetPoint` (`self.P_BarLine4`) 0 (`self.K2_GetActorLocation` (`self.Character`)) 0)
  (`ParticleSystemComponent.SetBeamTargetPoint` (`self.P_BarLine5`) 0 (`self.K2_GetActorLocation` (`self.Character`)) 0)
  (`ParticleSystemComponent.SetBeamTargetPoint` (`self.P_BarLine6`) 0 (`self.K2_GetActorLocation` (`self.Character`)) 0)
  (`ParticleSystemComponent.SetBeamTargetPoint` (`self.P_BarLine7`) 0 (`self.K2_GetActorLocation` (`self.Character`)) 0)
  (`ParticleSystemComponent.SetBeamTargetPoint` (`self.P_BarLine8`) 0 (`self.K2_GetActorLocation` (`self.Character`)) 0)
  (`ParticleSystemComponent.SetBeamTargetPoint` (`self.P_BarLine9`) 0 (`self.K2_GetActorLocation` (`self.Character`)) 0)
  (`ParticleSystemComponent.SetBeamSourcePoint` _p_barline 0 (0.0 0.0 0.0) 0)
  (`ParticleSystemComponent.SetBeamSourcePoint` (`self.P_BarLine2`) 0 (0.0 0.0 0.0) 0)
  (`ParticleSystemComponent.SetBeamSourcePoint` (`self.P_BarLine3`) 0 (0.0 0.0 0.0) 0)
  (`ParticleSystemComponent.SetBeamSourcePoint` (`self.P_BarLine4`) 0 (0.0 0.0 0.0) 0)
  (`ParticleSystemComponent.SetBeamSourcePoint` (`self.P_BarLine6`) 0 (0.0 0.0 0.0) 0)
  (`ParticleSystemComponent.SetBeamSourcePoint` (`self.P_BarLine7`) 0 (0.0 0.0 0.0) 0)
  (`ParticleSystemComponent.SetBeamSourcePoint` (`self.P_BarLine9`) 0 (0.0 0.0 0.0) 0)
  (if (>= (`/Game/Player/BP_PlayerController.TakeOverCounter` (`self.TakeOverCounter`)) 7.0)
    (for _array_element (`|MakeArray` (`self.P_BarLine`) (`self.P_BarLine2`) (`self.P_BarLine3`) (`self.P_BarLine4`) (`self.P_BarLine5`) (`self.P_BarLine6`) null (`self.P_BarLine7`) (`self.P_BarLine8`) (`self.P_BarLine9`))
      (`SceneComponent.SetVisibility` _array_element (`self.VisibilityOn`) false))
    (elif (>= (`/Game/Player/BP_PlayerController.TakeOverCounter` (`self.TakeOverCounter`)) 5.0)
      (for _array_element_2 (`|MakeArray` (`self.P_BarLine`) (`self.P_BarLine2`) (`self.P_BarLine3`) (`self.P_BarLine4`))
        (`SceneComponent.SetVisibility` _array_element_2 (`self.VisibilityOn`) false)
        (for _array_element_3 (`|MakeArray` (`self.P_BarLine5`) (`self.P_BarLine6`) (`self.P_BarLine7`) (`self.P_BarLine8`) (`self.P_BarLine9`))
          (`SceneComponent.SetVisibility` _array_element_3 (`self.VisibilityOff`) false)))
      (elif (>= (`/Game/Player/BP_PlayerController.TakeOverCounter` (`self.TakeOverCounter`)) 5.0)
        (`SceneComponent.SetVisibility` (`self.P_BarLine`) (`self.VisibilityOn`) false)
        (for _array_element_4 (`|MakeArray` (`self.P_BarLine2`) (`self.P_BarLine3`) (`self.P_BarLine4`) (`self.P_BarLine5`) (`self.P_BarLine6`) (`self.P_BarLine7`) (`self.P_BarLine8`) (`self.P_BarLine9`) null)
          (`SceneComponent.SetVisibility` _array_element_4 (`self.VisibilityOff`) false))))))

(fn `UserConstructionScript`)