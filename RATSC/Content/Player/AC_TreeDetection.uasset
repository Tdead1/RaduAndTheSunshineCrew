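; Player component on BP_CameraController that picks and highlights the tree the player is most facing.
; Every tick it gathers trees overlapping the player capsule, skips the current one, and compares each one's yaw from the owner against the follow arrow's forward yaw.
; The smallest raw yaw difference, without angle wrapping, becomes ClosestTree and turns transparent blue, after all overlapping trees reset to the basic wall material.
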(event `self.ReceiveBeginPlay`
  (bind _asbp_camera_controller (cast `/Game/Player/BP_CameraController` (`self.GetOwner`)))
  (set `self.Owner` _asbp_camera_controller))

(event `self.ReceiveTick`
  (params (DeltaSeconds :type "Float (single-precision)"))
  (bind (_returnvalue_roll _returnvalue_pitch _returnvalue_yaw) (`KismetMathLibrary.BreakRotator` (`KismetMathLibrary.FindLookAtRotation` (0.0 0.0 0.0) (`SceneComponent.GetForwardVector` (`self.ArrowComponentToFollow`)))))
  (switch `/Game/Player/E_PlayerState` (`self.PlayerState`)
    (:`NewEnumerator0`
      _)
    (:`NewEnumerator1`
      _)
    (:`NewEnumerator2`
      _))
  (bind _output_get (set `self.PossibleTrees` (`PrimitiveComponent.GetOverlappingActors` (`self.PlayerCapsuleCollider`) "/Game/AI/BP_Tree.BP_Tree_C")))
  (for _array_element _output_get
    (if (not (== _array_element (`self.CurrentActor`)))
      (bind (_returnvalue_roll_2 _returnvalue_pitch_2 _returnvalue_yaw_2) (`KismetMathLibrary.BreakRotator` (`KismetMathLibrary.FindLookAtRotation` (`Actor.K2_GetActorLocation` (`self.Owner`)) (`Actor.K2_GetActorLocation` _array_element))))
      (bind _returnvalue (`KismetMathLibrary.Abs` (- _returnvalue_yaw_2 _returnvalue_yaw)))
      (if (< _returnvalue (`self.ClosestAngle`))
        (set `self.ClosestAngle` _returnvalue)
        (bind _asbp_tree (cast `/Game/AI/BP_Tree` _array_element))
        (set `self.TempClosest` _asbp_tree))))
  (for _array_element_2 _output_get
    (bind _asbp_tree_2 (cast `/Game/AI/BP_Tree` _array_element_2))
    (`PrimitiveComponent.SetMaterial` (`/Game/AI/BP_Tree.Cylinder` _asbp_tree_2) 0 "/Game/StarterContent/Materials/M_Basic_Wall.M_Basic_Wall"))
  (bind _output_get_2 (set `self.ClosestTree` (`self.TempClosest`)))
  (`PrimitiveComponent.SetMaterial` (`/Game/AI/BP_Tree.Cylinder` _output_get_2) 0 "/Game/Materials/Whisps/M_BlueTransparent.M_BlueTransparent")
  (set `self.ClosestAngle` 360.0))