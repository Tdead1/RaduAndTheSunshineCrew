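; BP_PlayerMeshHolder drives the player's skeletal mesh through dash and idle animations.
; UpdateAnimation plays DashStart, then switches to DashLoop after a short delay if its gate is still open.
; Tick polls the player controller's LerpValue, closing the gate near the end and playing DashStart backwards once as the dash exit.
; When LerpValue is almost complete, a brief delay leads into the looping idle.
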(event `self.ReceiveBeginPlay`
  (set `self.PlayerController` (cast `/Game/Player/BP_PlayerController` (`GameplayStatics.GetPlayerController` 0) :!pure true)))

(event `UpdateAnimation`
  (switch `/Game/Player/E_PlayerState` "NewEnumerator2"
    (:`NewEnumerator2`
      (`|ExecutionSequence`
        (:`then_0`
          (`SkeletalMeshComponent.PlayAnimation` (`self.SkeletalMesh`) "/Game/Player/dashStart.dashStart" false)
          (`SkeletalMeshComponent.SetPlayRate` (`self.SkeletalMesh`) 1.0)
          (`KismetSystemLibrary.Delay` 0.35)
          (`/Engine/EditorBlueprintResources/StandardMacros.Gate` true :!label _label
            (:`Exit`
              (`SkeletalMeshComponent.PlayAnimation` (`self.SkeletalMesh`) "/Game/Player/dashLoop.dashLoop" true)
              (`SkeletalMeshComponent.SetPlayRate` (`self.SkeletalMesh`) 1.0))))
        (:`then_1`
          (goto _label :!via `Open`))
        (:`then_2`
          (goto _label_2 :!via `Reset`))))))

(event `self.ReceiveTick`
  (params (DeltaSeconds :type "Float (single-precision)"))
  (bind _lerpvalue (`/Game/Player/BP_PlayerController.LerpValue` (`self.PlayerController`)))
  (`|ExecutionSequence`
    (:`then_0`
      (if (> _lerpvalue 0.8)
        (`|ExecutionSequence`
          (:`then_0`
            (goto _label :!via `Close`))
          (:`then_1`
            (`/Engine/EditorBlueprintResources/StandardMacros.DoOnce` false :!label _label_2
              (:`Completed`
                (`SkeletalMeshComponent.Stop` (`self.SkeletalMesh`))
                (`SkeletalMeshComponent.SetAnimation` (`self.SkeletalMesh`) "/Game/Player/dashStart.dashStart")
                (`SkeletalMeshComponent.SetPosition` (`self.SkeletalMesh`) 1.0 true)
                (`SkeletalMeshComponent.SetPlayRate` (`self.SkeletalMesh`) -1.0)
                (`SkeletalMeshComponent.Play` (`self.SkeletalMesh`) false)))))))
    (:`then_1`
      (if (`KismetMathLibrary.NearlyEqual_FloatFloat` _lerpvalue 1.0 0.05)
        (`KismetSystemLibrary.Delay` 0.2)
        (`SkeletalMeshComponent.PlayAnimation` (`self.SkeletalMesh`) "/Game/Player/idle_Anim.idle_Anim" true)
        (`SkeletalMeshComponent.SetPlayRate` (`self.SkeletalMesh`) 1.0)))))

(fn `UserConstructionScript`)