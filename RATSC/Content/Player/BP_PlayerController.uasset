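; Player controller that flies the view between a big tree (the player pawn) and smaller trees.
; On begin play it spawns the camera controller, mesh holder, in-game UI and wind loop; the mouse rotates the camera.
; Clicking targets the closest detected tree; Tick moves the camera along a spline with FOV, speed-line and wind effects, trailed by the mesh.
; Small-tree perches drain the exit bar; timeout or Space returns to the big tree.
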(event `self.ReceiveBeginPlay`
  (bind _currentpawn (`self.CurrentPawn`))
  (bind (_cameraoffset_x _cameraoffset_y _cameraoffset_z) (`KismetMathLibrary.BreakVector` (`self.CameraOffset`)))
  (bind (_returnvalue_x _returnvalue_y) (`KismetMathLibrary.BreakVector` (* (`self.GetActorForwardVector` _currentpawn) _cameraoffset_x)))
  ;[1 1 1] Events
  (`|ExecutionSequence`
    (:`then_0`
      ;[1 1 1] BeginPlay
      (set `self.CurrentPawn` (`GameplayStatics.GetPlayerPawn` 0))
      (bind _output_get (set `self.TargetPosition` (`KismetMathLibrary.MakeTransform` (+ (`self.K2_GetActorLocation` _currentpawn) (`KismetMathLibrary.MakeVector` _returnvalue_x _returnvalue_y _cameraoffset_z)) (`self.K2_GetActorRotation` (`self.CurrentPawn`)))))
      (bind _output_get_2 (set `self.StartPosition` _output_get))
      (bind _returnvalue (`|SpawnActorFromClass` "/Game/Player/BP_CameraController.BP_CameraController_C" _output_get_2 "Undefined" "OverrideRootScale" null null))
      (bind _output_get_3 (set `self.PlayerCamManager` _returnvalue))
      (set `/Game/Player/BP_CameraController.ControllerRef` self _output_get_3)
      (`self.SetViewTargetWithBlend` _output_get_3)
      (set `SpringArmComponent.TargetArmLength` (`self.CameraBoomLength`) (`/Game/Player/BP_CameraController.SpringArm` (`self.PlayerCamManager`)))
      (bind _returnvalue_2 (`|SpawnActorFromClass` "/Game/Player/BP_PlayerMeshHolder.BP_PlayerMeshHolder_C" (`self.GetTransform` (`self.PlayerCamManager`)) "Undefined" "OverrideRootScale" null null))
      (bind _output_get_4 (set `self.PlayerMeshHolder` _returnvalue_2))
      (set `/Game/Player/AC_TreeDetection.PlayerCapsuleCollider` (`/Game/Player/BP_PlayerMeshHolder.Capsule` _output_get_4) (`/Game/Player/BP_CameraController.AC_TreeDetection` (`self.PlayerCamManager`))))
    (:`then_1`
      ;[1 1 1] UI setup and Audio
      (bind _returnvalue_3 (`|CreateWidget` "/Game/UI/W_InGameUI.W_InGameUI_C" self))
      (bind _output_get_5 (set `self.InGameUI` _returnvalue_3))
      (`UserWidget.AddToViewport` _output_get_5 0)
      (bind _returnvalue_4 (`GameplayStatics.CreateSound2D` "/Game/Audio/windblow_loop.windblow_loop"))
      (bind _output_get_6 (set `self.WindSound` _returnvalue_4))
      (`AudioComponent.Play` _output_get_6 0.0))))

(event `InputAxisKey|MouseX`
  (params (AxisValue :type "Float (single-precision)"))
  (bind _playercammanager (`self.PlayerCamManager`))
  ;[1 1 1] Process Input
  ;;[1 1 1] Mouse X
  (`self.K2_SetActorRotation` _playercammanager (`KismetMathLibrary.Conv_VectorToRotator` (`KismetMathLibrary.RotateAngleAxis` (`KismetMathLibrary.Conv_RotatorToVector` (`self.K2_GetActorRotation` _playercammanager)) AxisValue (`self.GetActorUpVector` _playercammanager))) false))

(event `InputAxisKey|MouseY`
  (params (AxisValue :type "Float (single-precision)"))
  (bind _playercammanager (`self.PlayerCamManager`))
  ;[1 1 1] Process Input
  ;;[1 1 1] Mouse Y
  (`self.K2_SetActorRotation` _playercammanager (`KismetMathLibrary.Conv_VectorToRotator` (`KismetMathLibrary.RotateAngleAxis` (`KismetMathLibrary.Conv_RotatorToVector` (`self.K2_GetActorRotation` _playercammanager)) (* AxisValue -1.0) (`self.GetActorRightVector` _playercammanager))) false))

(event `self.ReceiveTick`
  (params (DeltaSeconds :type "Float (single-precision)"))
  (bind _startposition_location (`KismetMathLibrary.BreakTransform` (`self.StartPosition`)))
  (bind _targetposition_location (`KismetMathLibrary.BreakTransform` (`self.TargetPosition`)))
  (bind _playercammanager (`self.PlayerCamManager`))
  (bind _targetactor (`self.TargetActor`))
  (bind _startposition_location_2 (`KismetMathLibrary.BreakTransform` (`self.StartPosition`)))
  (bind _targetposition_location_2 (`KismetMathLibrary.BreakTransform` (`self.TargetPosition`)))
  (bind _currentpawn (`self.CurrentPawn`))
  (bind (_cameraoffset_x _cameraoffset_y _cameraoffset_z) (`KismetMathLibrary.BreakVector` (`self.CameraOffset`)))
  (bind (_cameraoffset_x_2 _cameraoffset_y_2 _cameraoffset_z_2) (`KismetMathLibrary.BreakVector` (`self.CameraOffset`)))
  (bind _lerpvalue (`self.LerpValue`))
  (bind (_startposition_location_3 _startposition_rotation) (`KismetMathLibrary.BreakTransform` (`self.StartPosition`)))
  (bind (_targetposition_location_3 _targetposition_rotation) (`KismetMathLibrary.BreakTransform` (`self.TargetPosition`)))
  (bind _playercammanager_2 (`self.PlayerCamManager`))
  (bind (_returnvalue_location _returnvalue_rotation _returnvalue_scale) (`KismetMathLibrary.BreakTransform` (`self.GetTransform` (`self.TargetActor`))))
  (bind (_asbp_tree _bsuccess) (cast `/Game/AI/BP_Tree` (`self.TargetActor`) :!pure true))
  (bind (_asbp_tree_2 _bsuccess_2) (cast `/Game/AI/BP_Tree` (`self.TargetActor`) :!pure true))
  (bind _maincamera (`/Game/Player/BP_CameraController.MainCamera` _playercammanager_2))
  (bind _fovstandard (`/Game/Player/BP_CameraController.FOVStandard` _playercammanager_2))
  (bind _fovmoving (`/Game/Player/BP_CameraController.FOVMoving` _playercammanager_2))
  (bind _spline (`/Game/Player/BP_CameraController.Spline` (`self.PlayerCamManager`)))
  (bind _speedlinesfx (`/Game/Player/BP_CameraController.SpeedLinesFX` _playercammanager_2))
  (bind (_returnvalue_x _returnvalue_y) (`KismetMathLibrary.BreakVector` (* (`self.GetActorRightVector` _playercammanager) _cameraoffset_x)))
  (bind _returnvalue_location_2 (`KismetMathLibrary.BreakTransform` (`SplineComponent.GetTransformAtTime` _spline (`self.LerpValue`) "World" false false)))
  (bind (_returnvalue_x_2 _returnvalue_y_2) (`KismetMathLibrary.BreakVector` (* (`self.GetActorForwardVector` _currentpawn) _cameraoffset_x_2)))
  (bind _returnvalue (+ (`self.K2_GetActorLocation` _currentpawn) (`KismetMathLibrary.MakeVector` _returnvalue_x_2 _returnvalue_y_2 _cameraoffset_z_2)))
  (bind _returnvalue_2 (+ _returnvalue_location (`KismetMathLibrary.MakeVector` _returnvalue_x _returnvalue_y _cameraoffset_z)))
  (bind _returnvalue_3 (select `bool` (< _lerpvalue 0.5) :`false` (* (- 1.0 _lerpvalue) 2.0) :`true` (* _lerpvalue 2.0)))
  ;[1 1 1] Events
  (`|ExecutionSequence`
    (:`then_1`
      ;[1 1 1] Camera Location
      (if (`self.IsSwitchingTarget`)
        (`|ExecutionSequence`
          (:`then_0`
            ;[1 1 1] Setting up start points and end points
            (`/Engine/EditorBlueprintResources/StandardMacros.DoOnce` false :!label _label
              (:`Completed`
                (set `self.StartPosition` (`self.GetTransform` _playercammanager))
                (set `self.TargetPosition` (`KismetMathLibrary.MakeTransform` (`KismetMathLibrary.SelectVector` (+ _returnvalue_2 (`/Game/AI/BP_Tree.PerchLocation` _asbp_tree_2)) _returnvalue_2 _bsuccess_2) (`self.K2_GetActorRotation` _playercammanager) _returnvalue_scale)))))
          (:`then_1`
            ;[1 1 1] Doing the movement
            (set `self.CurrentState` "NewEnumerator2")
            (`SplineComponent.SetSplinePoints` _spline (`|MakeArray` _startposition_location_3 _targetposition_location_3) "World" true)
            (`self.K2_SetActorTransform` (`self.PlayerCamManager`) (`KismetMathLibrary.MakeTransform` _returnvalue_location_2 (`KismetMathLibrary.RLerp` _startposition_rotation _targetposition_rotation (`self.LerpValue`))) false false)
            (bind _output_get (set `self.LerpValue` (`KismetMathLibrary.FClamp` (+ (* (`GameplayStatics.GetWorldDeltaSeconds`) (/ (`self.CameraFlySpeed`) (`KismetMathLibrary.VSize` (- _targetposition_location _startposition_location)))) (`self.LerpValue`)))))
            ;[1 1 1] When the movement is done...
            (if (`KismetMathLibrary.NearlyEqual_FloatFloat` _output_get 1.0 0.01)
              (`MaterialInstanceDynamic.SetScalarParameterValue` _speedlinesfx "Weight" 0.0)
              (`CameraComponent.SetFieldOfView` _maincamera (`KismetMathLibrary.Lerp` _fovstandard _fovmoving _returnvalue_3))
              (set `self.IsSwitchingTarget` false)
              (set `self.CurrentPawn` _targetactor)
              (bind _asbp_tree_3 (cast `/Game/AI/BP_Tree` _targetactor)
                (:`then`
                  (`/Game/AI/BP_Tree.Boom` _asbp_tree_3))
                (:`CastFailed`
                  _))
              (set `self.LerpValue` 0.0)
              (set `self.IsCountingDown` true)
              (goto _label :!via `Reset`)
              (else
                (`MaterialInstanceDynamic.SetScalarParameterValue` _speedlinesfx "Weight" 1.0)
                (`CameraComponent.SetFieldOfView` _maincamera (`KismetMathLibrary.Lerp` _fovstandard _fovmoving _returnvalue_3))))))
        (else
          (`self.K2_SetActorLocation` (`self.PlayerCamManager`) (`KismetMathLibrary.SelectVector` (+ _returnvalue (`/Game/AI/BP_Tree.PerchLocation` _asbp_tree)) _returnvalue _bsuccess) false false)
          ;[1 1 1] Count down timer for AI takeovers
          (if (`self.IsCountingDown`)
            (if (`self.IsAtBigTree`)
              (set `self.CurrentState` "NewEnumerator0")
              (else
                (bind _output_get_2 (set `self.TakeOverCounter` (`KismetMathLibrary.FClamp` (- (`self.TakeOverCounter`) (/ (`GameplayStatics.GetWorldDeltaSeconds`) (`self.SecondsAllowedInTarget`))) 0.0 10000.0)))
                (set `self.CurrentState` "NewEnumerator1")
                (if (`KismetMathLibrary.NearlyEqual_FloatFloat` _output_get_2 0.0 0.0001)
                  (`self.GoBackToTree`))
                (`ProgressBar.SetPercent` (`/Game/UI/W_InGameUI.ExitBar` (`self.InGameUI`)) (`self.TakeOverCounter`))))))))
    (:`then_2`
      ;[1 1 1] Set Mesh Location
      (switch `/Game/Player/E_PlayerState` (`self.CurrentState`)
        (:`NewEnumerator0`
          _)
        (:`NewEnumerator1`
          _)
        (:`NewEnumerator2`
          _))
      (`self.K2_SetActorTransform` (`self.PlayerMeshHolder`) (`KismetMathLibrary.MakeTransform` (`self.K2_GetActorLocation` (`self.PlayerCamManager`)) (`KismetMathLibrary.Conv_VectorToRotator` (`KismetMathLibrary.Normal` (- _targetposition_location_2 _startposition_location_2))) (1.0 1.0 1.0)) false false))
    (:`then_3`
      ;[1 1 1] Audio volume settings, and setup components of the camera
      (`AudioComponent.SetVolumeMultiplier` (`self.WindSound`) (`self.LerpValue`))
      (set `/Game/Player/AC_TreeDetection.CurrentActor` (`self.TargetActor`) (`/Game/Player/BP_CameraController.AC_TreeDetection` (`self.PlayerCamManager`))))))

(event `Key|LeftMouseButton`
  (params (Key :type "Key Structure"))
  ;[1 1 1] Events
  (:`Pressed`
    (switch `/Game/Player/E_PlayerState` (`self.CurrentState`)
      (:`NewEnumerator0`
        _)
      (:`NewEnumerator1`
        _))
    ;[1 1 1] Setting up targets for switching (by clicking)
    (set `self.TargetActor` (`/Game/Player/AC_TreeDetection.ClosestTree` (`/Game/Player/BP_CameraController.AC_TreeDetection` (`self.PlayerCamManager`))))
    (set `self.IsSwitchingTarget` true)
    (`/Game/Player/BP_PlayerMeshHolder.UpdateAnimation` (`self.PlayerMeshHolder`))
    (set `self.IsAtBigTree` false)))

(event `GoBackToTree`
  ;[1 1 1] Events
  ;[1 1 1] Moving back to the main tree.
  (set `SpringArmComponent.TargetArmLength` (`self.CameraBoomLength`) (`/Game/Player/BP_CameraController.SpringArm` (`self.PlayerCamManager`)))
  (set `self.TargetActor` (`GameplayStatics.GetPlayerPawn` 0))
  (set `self.IsSwitchingTarget` true)
  (set `self.IsAtBigTree` true)
  (set `self.TakeOverCounter` 1.0)
  (goto _label :!via `Reset`))

(event `Key|SpaceBar`
  (params (Key :type "Key Structure"))
  ;[1 1 1] Events
  (:`Pressed`
    ;[1 1 1] Moving back to the main tree.
    (`self.GoBackToTree`)))

(fn `UserConstructionScript`)