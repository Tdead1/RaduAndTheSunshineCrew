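; Player camera controller that hosts tree detection and a speed-lines post-process effect.
; On BeginPlay it hands its Arrow to the ACTreeDetection component to follow and adds a dynamic speed-lines material to PostProcess at full weight, keeping it in SpeedLinesFX.
; Every Tick it copies the current state from BP_PlayerController into the tree detection component.
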(event `self.ReceiveBeginPlay`
  (set `/Game/Player/AC_TreeDetection.ArrowComponentToFollow` (`self.Arrow`) (`self.AC_TreeDetection`))
  (bind _returnvalue (`KismetMaterialLibrary.CreateDynamicMaterialInstance` "/Game/Player/CameraFX/M_Speedlines.M_Speedlines"))
  (`PostProcessComponent.AddOrUpdateBlendable` (`self.PostProcess`) _returnvalue 1.0)
  (set `self.SpeedLinesFX` _returnvalue))

(event `self.ReceiveTick`
  (params (DeltaSeconds :type "Float (single-precision)"))
  (set `/Game/Player/AC_TreeDetection.PlayerState` (`/Game/Player/BP_PlayerController.CurrentState` (cast `/Game/Player/BP_PlayerController` (`GameplayStatics.GetPlayerController` 0) :!pure true)) (`self.AC_TreeDetection`)))

(fn `UserConstructionScript`)