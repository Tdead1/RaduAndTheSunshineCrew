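; BP_TakeOverCharacter is an AI-driven character that seeds its controller's Blackboard with its identity and starting state.
; On BeginPlay it caches its AI controller, then writes itself to the SelfActor key and its State variable to the State key.
; Two small helper functions wrap the Blackboard object and enum writes; the file itself holds no further behavior logic.
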(event `self.ReceiveBeginPlay`
  (set `self.AIController` (`AIBlueprintHelperLibrary.GetAIController` self))
  (`self.Set Self Actor` "SelfActor" self)
  (`self.Set State` "State" (`self.State`)))

(fn `Set Self Actor`
  (params (`Key Name` :type Name) (`Self Actor` :type "Object Object Reference"))
  (`BlackboardComponent.SetValueAsObject` (`AIBlueprintHelperLibrary.GetBlackboard` (`self.AIController`)) `Key Name` `Self Actor`))

(fn `Set State`
  (params (`Key Name` :type Name) (State :type "/Game/AI/E_TakeOverCharacterState Enum" :default "NewEnumerator0"))
  (`BlackboardComponent.SetValueAsEnum` (`AIBlueprintHelperLibrary.GetBlackboard` (`self.AIController`)) `Key Name` State))

(fn `UserConstructionScript`)