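; BP_TreeManager is an AI-folder manager that keeps an array of records for every BP_Tree in the level.
; On BeginPlay it stores each tree's default HP, world chop location and actor reference.
; SelectRandomName feeds the name field but is never executed; it also removes a separately rolled entry, with an out-of-range maximum index.
; UpdateState rewrites a record with a new state, preserving its other fields.
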(event EventBeginPlay
  (bind _outactors (Actor|GetAllActorsOfClass "/Game/AI/BP_Tree.BP_Tree_C"))
  (for (_array_element _array_index) _outactors
    (Utilities|Array|SetArrayElem (Variables|Default|GetTreeArray) _array_index (Utilities|Struct|MakeD_Tree (stale _name) "NewEnumerator0" (Variables|Default|GetDefaultTreeHP) (+ (Variables|/Game/AI/BP_Tree.BP_Tree_C|GetChopLocation _array_element) (Transformation|GetActorLocation _array_element)) _array_element) true)))

(fn ConstructionScript)

(fn SelectRandomName
  (bind _names (Variables|Default|GetNames))
  (bind _returnvalue (Utilities|Array|Length _names))
  (bind _returnvalue_2 (Math|Random|RandomIntegerinRange 0 _returnvalue))
  (bind _output (Utilities|Array|Get(acopy) _names _returnvalue_2))
  (LocalVariables|SetLocalName _output)
  (Utilities|Array|RemoveItem _names _output)
  (return (LocalVariables|GetLocalName)))

(fn UpdateState
  (params (State :type E_TreeState%20Enum :default "NewEnumerator0") (Tree%20Index :type Integer))
  (bind _treearray (Variables|Default|GetTreeArray))
  (bind _output (Utilities|Array|Get(acopy) _treearray Tree%20Index))
  (Utilities|Array|SetArrayElem (Variables|Default|GetTreeArray) Tree%20Index (Utilities|Struct|MakeD_Tree (.name _output) State (.hp _output) (.location _output) (.selfactor _output)) true))