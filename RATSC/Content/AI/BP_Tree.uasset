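; BP_Tree is a tree actor that can be destroyed or set off as an explosion that kills nearby characters.
; The construction script picks the static mesh from Type, though Normal and PowerUp both currently use TreeSmall.
; RIP destroys the tree, while Boom destroys every BP_TakeOverCharacter overlapping its Sphere and spawns a heavily scaled explosion emitter.
; Boom does not destroy the tree itself, and neither event is called within this Blueprint.
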(event `RIP`
  (`self.K2_DestroyActor`))

(event `Boom`
  (bind (_returnvalue_location _returnvalue_rotation) (`KismetMathLibrary.BreakTransform` (`self.GetTransform`)))
  (for _array_element (`PrimitiveComponent.GetOverlappingActors` (`self.Sphere`) "/Game/AI/BP_TakeOverCharacter.BP_TakeOverCharacter_C")
    (`self.K2_DestroyActor` _array_element))
  (`GameplayStatics.SpawnEmitterAtLocation` (`self.ExplosionEffect`) _returnvalue_location _returnvalue_rotation (100.0 100.0 100.0)))

(fn `UserConstructionScript`
  (`StaticMeshComponent.SetStaticMesh` (`self.StaticMesh`) (select `/Game/AI/E_TreeType` (`self.Type`) :`NewEnumerator0` "/Game/Art/ArtAssets/treeSmall.treeSmall" :`NewEnumerator1` "/Game/Art/ArtAssets/treeSmall.treeSmall" :!type "StaticMesh Object Reference")))