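; BP_ScoreAndPowerUps keeps a frame-driven score and spawns lightning power-up pickups on trees.
; On BeginPlay it caches the first BP_TreeManager in the level.
; Each Tick increments and prints the score, then calls SpawnPowerup.
; At every multiple of 50, that event scans the manager's TreeArray and spawns BP_LightingPower at the perch point of every tree matching one enum type.
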(event `self.ReceiveTick`
  (params (DeltaSeconds :type "Float (single-precision)"))
  (`/Engine/EditorBlueprintResources/StandardMacros.IncrementInt` (`self.Score`)
    (:`  `
      (`self.Spawn Powerup`)
      (`KismetSystemLibrary.PrintString` (`KismetStringLibrary.Conv_IntToString` (`self.Score`)) true true (struct :`G` 0.66 :`B` 1.0 :`A` 1.0) (`GameplayStatics.GetWorldDeltaSeconds`)))))

(event `self.ReceiveBeginPlay`
  (bind _outactors (`GameplayStatics.GetAllActorsOfClass` "/Game/AI/BP_TreeManager.BP_TreeManager_C"))
  (set `self.Tree Manager` (`|GetArrayItem` _outactors)))

(event `Spawn Powerup`
  (if (== (mod (`self.Score`) 50) 0)
    (for _array_element (`/Game/AI/BP_TreeManager.TreeArray` (`self.Tree Manager`))
      (if (`|EnumEquality` (`.Type_19_855258634263D70372D980A47B46348E` (break `/Game/AI/D_Tree` _array_element)) "NewEnumerator1")
        (`KismetSystemLibrary.PrintString` (`KismetStringLibrary.Conv_VectorToString` (`.Location_12_950239A343E3994D07D2579C39DED009` (break `/Game/AI/D_Tree` _array_element))))
        (`|SpawnActorFromClass` "/Game/AI/BP_LightingPower.BP_LightingPower_C" (`KismetMathLibrary.MakeTransform` (+ (`self.K2_GetActorLocation` (`.SelfActor_15_48848D014B60A236AA5B8199A8EE0911` (break `/Game/AI/D_Tree` _array_element))) (`/Game/AI/BP_Tree.PerchLocation` (`.SelfActor_15_48848D014B60A236AA5B8199A8EE0911` (break `/Game/AI/D_Tree` _array_element))))) "Undefined" "OverrideRootScale" null null)))))

(fn `UserConstructionScript`)