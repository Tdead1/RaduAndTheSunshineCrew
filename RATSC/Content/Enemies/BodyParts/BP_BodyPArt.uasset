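; Enemy body part actor that appears as a random mesh and gets pulled toward the player as a physics object.
; BeginPlay picks one of the meshes in StaticMeshParts, enables physics simulation and opens a gate on Tick.
; Through a FlipFlop, every other tick applies a negative-strength, constant-falloff radial impulse centered on the player controller's PlayerMeshHolder, drawing the part in.
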(event `self.ReceiveTick`
  (params (DeltaSeconds :type "Float (single-precision)"))
  (`/Engine/EditorBlueprintResources/StandardMacros.Gate` true :!label _label
    (:`Exit`
      (`/Engine/EditorBlueprintResources/StandardMacros.FlipFlop`
        (:`A`
          (`PrimitiveComponent.AddRadialImpulse` (`self.StaticMesh`) (`self.K2_GetActorLocation` (`/Game/Player/BP_PlayerController.PlayerMeshHolder` (cast `/Game/Player/BP_PlayerController` (`GameplayStatics.GetPlayerController` 0) :!pure true))) 50000.0 -1000.0 "RIF_Constant" false))))))

(event `self.ReceiveBeginPlay`
  (`StaticMeshComponent.SetStaticMesh` (`self.StaticMesh`) (`|GetArrayItem` (`self.StaticMeshParts`) (`KismetMathLibrary.RandomInteger` 17)))
  (`PrimitiveComponent.SetSimulatePhysics` (`self.StaticMesh`) true)
  (goto _label :!via `Open`))

(fn `UserConstructionScript`)